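; Collectible coin pickup for a runner game that adds to the coin count when the player touches it.
; Tick spins the Coin component on its local roll axis at RotationSpeed, scaled by delta time.
; On overlap with an actor tagged Player, it calls AddCoin on RunnerGamemode and destroys itself.
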(event `self.ReceiveTick`
  (params (DeltaSeconds :type "Float (single-precision)"))
  (`SceneComponent.K2_AddLocalRotation` (`self.Coin`) (`KismetMathLibrary.MakeRotator` (* (`self.RotationSpeed`) DeltaSeconds)) false false))

(event `self.ReceiveActorBeginOverlap`
  (params (OtherActor :type "Actor Object Reference"))
  (if (`self.ActorHasTag` OtherActor "Player")
    (bind _asrunner_gamemode (cast `/Game/Blueprints/RunnerGamemode` (`GameplayStatics.GetGameMode`)))
    (`/Game/Blueprints/RunnerGamemode.AddCoin` _asrunner_gamemode)
    (`self.K2_DestroyActor`)))

(fn `UserConstructionScript`)