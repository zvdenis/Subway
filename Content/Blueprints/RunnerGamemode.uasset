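; Game mode for a three-lane endless runner that generates the track as Meters grows and ramps character speed with distance, up to a cap.
; Each row is a three-bit lane mask, randomized against earlier rows and spawned at an advancing transform.
; Bitwise tests on recent rows place obstacles, coins and rare power-ups, with random moving obstacles later in the run.
; BeginPlay also creates the HUD and lays the opening rows.
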(event `self.ReceiveBeginPlay`
  (`self.InitValues`
    (:`out`
      (`self.PlacePlatforms` 7)
      (`self.PlacePlatforms` 7)
      (for _ (range 8)
        (`self.GenTriple`)))))

(event `self.ReceiveTick`
  (params (DeltaSeconds :type "Float (single-precision)"))
  (bind _lastplatformmeters (`self.LastPlatformMeters`))
  (bind _character (`self.character`))
  (bind _startspeed (`/Game/Blueprints/ThirdPersonCharacter.StartSpeed` _character))
  (`|ExecutionSequence`
    (:`then_0`
      (if (< _lastplatformmeters (- (`self.Meters`) 8))
        (set `self.LastPlatformMeters` (+ _lastplatformmeters 6))
        (`self.GenTriple`)))
    (:`then_1`
      (if (`self.GameStarted`)
        (set `/Game/Blueprints/ThirdPersonCharacter.CurSpeed` (`KismetMathLibrary.FClamp` (+ _startspeed (* (/ (`self.Meters`) 200) 0.02)) _startspeed (`/Game/Blueprints/ThirdPersonCharacter.MaxSpeed` _character)) _character)))))

(fn `AddCoin`
  (`/Engine/EditorBlueprintResources/StandardMacros.IncrementInt` (`self.Coins`)))

(fn `GenBonus`
  (bind _returnvalue (`KismetMathLibrary.RandomInteger` 100))
  (set `self.PlatformSum` 0)
  (for _index (range 3)
    (set `self.PlatformSum` (`KismetMathLibrary.Xor_IntInt` (`self.PlatformSum`) (`|GetArrayItem` (`self.LastTriples`) _index))))
  (for _index_2 (range 3)
    (bind _output (`|GetArrayItem` (`self.LinePow`) _index_2))
    (if (and (and (`KismetMathLibrary.Conv_IntToBool` (`KismetMathLibrary.And_IntInt` _output (`self.PlatformSum`))) (`KismetMathLibrary.Conv_IntToBool` (`KismetMathLibrary.And_IntInt` _output (`|GetArrayItem` (`self.LastTriples`) 1)))) (not (`KismetMathLibrary.Conv_IntToBool` (`KismetMathLibrary.And_IntInt` _output (`|GetArrayItem` (`self.LastTriples`))))))
      (if (< _returnvalue 94)
        (`self.PlaceCoin` _index_2 2)
        (elif (`KismetMathLibrary.Conv_IntToBool` (mod _returnvalue 2))
          (`self.PlaceSpeedDecrease` _index_2 2)
          (else
            (`self.PlaceImmuneObstacles` _index_2 2)))))))

(fn `GenMovingObstacle`
  (if (>= (`self.Meters`) 300)
    (if (>= 1 (`KismetMathLibrary.RandomInteger` 40))
      (`self.PlaceMovingObstacle` (`KismetMathLibrary.RandomInteger` 3)))))

(fn `GenObstacle`
  (bind _lasttriples (`self.LastTriples`))
  (set `self.PlatformSum` 7)
  (for _index (range 3)
    (set `self.PlatformSum` (`KismetMathLibrary.And_IntInt` (`self.PlatformSum`) (`|GetArrayItem` (`self.LastTriples`) _index))))
  (for _index_2 (range 3)
    (if (`KismetMathLibrary.Conv_IntToBool` (`KismetMathLibrary.And_IntInt` (`|GetArrayItem` (`self.LinePow`) _index_2) (`self.PlatformSum`)))
      (if (< (`KismetMathLibrary.RandomInteger` 2) 1)
        (`self.PlaceObstacle` _index_2 2)
        (`KismetArrayLibrary.Array_Set` _lasttriples 1 (- (`|GetArrayItem` _lasttriples 1) (`|GetArrayItem` (`self.LinePow`) _index_2)))))))

(fn `GenTriple`
  (`self.PlacePlatforms` (`KismetMathLibrary.Or_IntInt` (`KismetMathLibrary.Xor_IntInt` (+ (`KismetMathLibrary.RandomInteger` 6) 1) (`self.LastTriple`)) (`|GetArrayItem` (`self.LinePow`) (`KismetMathLibrary.RandomInteger` 4))))
  (`self.GenObstacle`)
  (`self.GenBonus`)
  (`self.GenMovingObstacle`))

(fn `MoveSpawnPoint`
  (bind _lasttriples (`self.LastTriples`))
  (set `self.NextSpawnPoint` (`KismetMathLibrary.MakeTransform` (+ (.location (`self.NextSpawnPoint`)) (600.0 0.0 0.0)) (.rotation (`self.NextSpawnPoint`)) (.scale (`self.NextSpawnPoint`))))
  (`KismetArrayLibrary.Array_Set` _lasttriples 2 (`|GetArrayItem` (`self.LastTriples`) 1))
  (`KismetArrayLibrary.Array_Set` _lasttriples 1 (`|GetArrayItem` (`self.LastTriples`)))
  (`KismetArrayLibrary.Array_Set` _lasttriples 0 (`self.CurTriple`))
  (set `self.CurTriple` 0))

(fn `PlaceActor`
  (params (Position :type Integer) (BackTo :type Integer) (ActorToPlace :type "Actor Class Reference"))
  (`|SpawnActorFromClass` ActorToPlace (`KismetMathLibrary.MakeTransform` (+ (.location (`self.NextSpawnPoint`)) (`KismetMathLibrary.MakeVector` (`KismetMathLibrary.Conv_IntToDouble` (* BackTo -600)) (* Position 300.0))) (.rotation (`self.NextSpawnPoint`)) (.scale (`self.NextSpawnPoint`))) "Undefined" "OverrideRootScale" null null))

(fn `PlaceCoin`
  (params (Position :type Integer) (BackTo :type Integer))
  (`self.PlaceActor` Position BackTo "/Game/Blueprints/Coin.Coin_C"))

(fn `PlaceImmuneObstacles`
  (params (Position :type Integer) (BackTo :type Integer))
  (`self.PlaceActor` Position BackTo "/Game/Blueprints/ObstaclesImmune.ObstaclesImmune_C"))

(fn `PlaceMovingObstacle`
  (params (Position :type Integer) (BackTo :type Integer))
  (`self.PlaceActor` Position BackTo "/Game/Blueprints/MovingObstacle.MovingObstacle_C"))

(fn `PlaceObstacle`
  (params (Position :type Integer) (BackTo :type Integer))
  (`self.PlaceActor` Position BackTo "/Game/Blueprints/Obstacle.Obstacle_C"))

(fn `PlacePlatform`
  (params (Position :type Integer))
  (`|SpawnActorFromClass` "/Game/Blueprints/Platform.Platform_C" (`KismetMathLibrary.MakeTransform` (+ (.location (`self.NextSpawnPoint`)) (`KismetMathLibrary.MakeVector` 0.0 (* (+ Position 1) 300.0))) (.rotation (`self.NextSpawnPoint`)) (.scale (`self.NextSpawnPoint`))) "Undefined" "OverrideRootScale" null null)
  (set `self.CurTriple` (+ (`self.CurTriple`) (`KismetMathLibrary.FTrunc` (`KismetMathLibrary.MultiplyMultiply_FloatFloat` 2.0 (`KismetMathLibrary.Conv_IntToDouble` (+ Position 1)))))))

(fn `PlacePlatforms`
  (params (Triple :type Integer))
  (if (`KismetMathLibrary.Conv_IntToBool` (`KismetMathLibrary.And_IntInt` Triple 1))
    (`self.PlacePlatform` -1))
  (if (`KismetMathLibrary.Conv_IntToBool` (`KismetMathLibrary.And_IntInt` Triple 2))
    (`self.PlacePlatform` 0))
  (if (`KismetMathLibrary.Conv_IntToBool` (`KismetMathLibrary.And_IntInt` Triple 4))
    (`self.PlacePlatform` 1))
  (`self.MoveSpawnPoint`))

(fn `PlaceSpeedDecrease`
  (params (Position :type Integer) (BackTo :type Integer))
  (`self.PlaceActor` Position BackTo "/Game/Blueprints/SpeedDecrease.SpeedDecrease_C"))

(fn `UserConstructionScript`)