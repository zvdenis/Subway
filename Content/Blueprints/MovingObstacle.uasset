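; Runner-game obstacle that moves along its local X axis and ends the run when it hits the player.
; Tick scales its speed by SpeedDecrease for 10 seconds after the slow pickup time stored on RunnerGamemode.
; A box overlap with a Player-tagged component sets GameOver, calls FinishRun on the character, fires impulse, particle and sound effects, then destroys the obstacle after a short delay.
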(event `self.ReceiveBeginPlay`
  (bind _asrunner_gamemode (cast `/Game/Blueprints/RunnerGamemode` (`GameplayStatics.GetGameMode`)))
  (set `self.GameMode` _asrunner_gamemode))

(event `self.ReceiveTick`
  (params (DeltaSeconds :type "Float (single-precision)"))
  (bind _defaultsceneroot (`self.DefaultSceneRoot`))
  (bind _returnvalue (* (`self.Speed`) DeltaSeconds))
  (bind _speeddecreaselastpicktime (`/Game/Blueprints/RunnerGamemode.SpeedDecreaseLastPickTime` (`self.GameMode`)))
  (if (`KismetMathLibrary.InRange_FloatFloat` (`GameplayStatics.GetTimeSeconds`) _speeddecreaselastpicktime (+ _speeddecreaselastpicktime 10.0))
    (`SceneComponent.K2_AddLocalOffset` _defaultsceneroot (`KismetMathLibrary.MakeVector` (* _returnvalue (`self.SpeedDecrease`))) false false)
    (else
      (`SceneComponent.K2_AddLocalOffset` _defaultsceneroot (`KismetMathLibrary.MakeVector` _returnvalue) false false))))

(event `self.Box.OnComponentBeginOverlap`
  (params (OverlappedComponent :type "PrimitiveComponent Object Reference") (OtherActor :type "Actor Object Reference") (OtherComp :type "PrimitiveComponent Object Reference") (OtherBodyIndex :type Integer) (bFromSweep :type Boolean) (SweepResult :type "HitResult Structure (by ref)"))
  (if (`ActorComponent.ComponentHasTag` OtherComp "Player")
    (set `/Game/Blueprints/RunnerGamemode.GameOver` true (`self.GameMode`))
    (bind _asthird_person_character (cast `/Game/Blueprints/ThirdPersonCharacter` (`GameplayStatics.GetPlayerCharacter` 0)))
    (`/Game/Blueprints/ThirdPersonCharacter.FinishRun` _asthird_person_character)
    (`self.Hit`)
    (`KismetSystemLibrary.Delay` 0.1)
    (`self.K2_DestroyActor`)))

(fn `Hit`
  (`RadialForceComponent.FireImpulse` (`self.RadialForce`))
  (`ActorComponent.Activate` (`self.ParticleSystem`) false)
  (`GameplayStatics.PlaySoundAtLocation` "/Game/StarterContent/Audio/Explosion01.Explosion01" (0.0 0.0 0.0) (struct) 0.5 1.0 0.0 null null null))

(fn `UserConstructionScript`)