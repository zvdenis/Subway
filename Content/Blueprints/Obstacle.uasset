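; Obstacle actor for a runner game that ends the run when the player touches it.
; Its box overlap checks for the Player tag, sets GameOver on RunnerGamemode, explodes with a radial impulse, particles and sound, then calls FinishRun on the character.
; Every tick it disables cube and box collision for ten seconds after the game mode's last obstacle-immunity pickup time, restoring it afterwards.
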(event `self.ReceiveBeginPlay`
  (bind _asrunner_gamemode (cast `/Game/Blueprints/RunnerGamemode` (`GameplayStatics.GetGameMode`)))
  (set `self.RunnerGameMode` _asrunner_gamemode))

(event `self.Box.OnComponentBeginOverlap`
  (params (OverlappedComponent :type "PrimitiveComponent Object Reference") (OtherActor :type "Actor Object Reference") (OtherComp :type "PrimitiveComponent Object Reference") (OtherBodyIndex :type Integer) (bFromSweep :type Boolean) (SweepResult :type "HitResult Structure (by ref)"))
  (if (`self.ActorHasTag` OtherActor "Player")
    (bind _asrunner_gamemode (cast `/Game/Blueprints/RunnerGamemode` (`GameplayStatics.GetGameMode`)))
    (set `/Game/Blueprints/RunnerGamemode.GameOver` true _asrunner_gamemode)
    (`self.Explode`)
    (bind _asthird_person_character (cast `/Game/Blueprints/ThirdPersonCharacter` (`GameplayStatics.GetPlayerCharacter` 0)))
    (`/Game/Blueprints/ThirdPersonCharacter.FinishRun` _asthird_person_character)))

(event `self.ReceiveTick`
  (params (DeltaSeconds :type "Float (single-precision)"))
  (bind _obstacleimmunelastpicktime (`/Game/Blueprints/RunnerGamemode.ObstacleImmuneLastPickTime` (`self.RunnerGameMode`)))
  (if (`KismetMathLibrary.InRange_FloatFloat` (`GameplayStatics.GetTimeSeconds`) _obstacleimmunelastpicktime (+ _obstacleimmunelastpicktime 10.0))
    (`PrimitiveComponent.SetCollisionEnabled` (`self.Cube`) "NoCollision")
    (`PrimitiveComponent.SetCollisionEnabled` (`self.Box`) "NoCollision")
    (else
      (`PrimitiveComponent.SetCollisionEnabled` (`self.Cube`) "QueryAndPhysics")
      (`PrimitiveComponent.SetCollisionEnabled` (`self.Box`) "QueryOnly"))))

(fn `Explode`
  (`RadialForceComponent.FireImpulse` (`self.RadialForce`))
  (`ActorComponent.Activate` (`self.ParticleSystem`) false)
  (`GameplayStatics.PlaySoundAtLocation` "/Game/StarterContent/Audio/Explosion01.Explosion01" (0.0 0.0 0.0) (struct) 0.5 1.0 0.0 null null null))

(fn `UserConstructionScript`)